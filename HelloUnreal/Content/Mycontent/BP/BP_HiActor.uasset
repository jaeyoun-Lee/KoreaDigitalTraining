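; BP_HiActor is a practice actor that moves its Sphere component back and forth along its relative X axis.
; Tick offsets the sphere by Speed scaled by delta time, and the IsTurn flag flips direction at fixed limits of 0 and 1000.
; BeginPlay and the overlap event are empty.
; Several disconnected node chains, such as print, loop, location and rotation tests, remain in the graph but never run.
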(event `self.ReceiveBeginPlay`)

(event `self.ReceiveTick`
  (params (DeltaSeconds :type "Float (single-precision)"))
  (bind _sphere (`self.Sphere`))
  (bind _sphere_2 (`self.Sphere`))
  (bind _relativelocation_x (`KismetMathLibrary.BreakVector` (`SceneComponent.RelativeLocation` _sphere)))
  (bind _relativelocation_x_2 (`KismetMathLibrary.BreakVector` (`SceneComponent.RelativeLocation` _sphere_2)))
  ;[0.8333 0.0246 0] 오른쪽 이동
  (if (`self.isTurn`)
    (`SceneComponent.K2_AddRelativeLocation` _sphere_2 (`KismetMathLibrary.MakeVector` (* DeltaSeconds (`self.Speed`))) false false)
    (if (>= _relativelocation_x_2 1000.0)
      (set `self.isTurn` false))
    (else
      ;[0 0.09904 1] 왼쪽 이동
      (`SceneComponent.K2_AddRelativeLocation` _sphere (`KismetMathLibrary.MakeVector` (* (* DeltaSeconds (`self.Speed`)) -1.0)) false false)
      (if (<= _relativelocation_x 0.0)
        (set `self.isTurn` true)))))

(event `self.Sphere.OnComponentBeginOverlap`
  (params (OverlappedComponent :type "PrimitiveComponent Object Reference") (OtherActor :type "Actor Object Reference") (OtherComp :type "PrimitiveComponent Object Reference") (OtherBodyIndex :type Integer) (bFromSweep :type Boolean) (SweepResult :type "HitResult Structure (by ref)")))

(fn `UserConstructionScript`)